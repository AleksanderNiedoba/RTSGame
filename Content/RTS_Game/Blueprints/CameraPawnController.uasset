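; RTS player controller that drives the camera pawn and handles building placement.
; On BeginPlay it caches references, spawns the construction manager and ghost building, and creates the main HUD.
; Camera supports zoom-scaled key movement, screen-edge scrolling, Shift boost, gated mouse pan/tilt and spring-arm zoom.
; In build mode the ghost follows the cursor, rotates, and queues construction on non-overlapping clicks; V spawns an NPC at the cursor.
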(event EventBeginPlay
  (bind _self self)
  (bind _defaultspawntransform (Variables|Default|GetDefaultSpawnTransform))
  ;[1 1 1] BeginPlay
  (Utilities|FlowControl|Sequence
    (:then_0
      (Utilities|ReferenceCasts))
    (:then_1
      (bind _returnvalue (Game|SpawnActorfromClass "/Game/RTS_Game/Blueprints/Construction/ConstructionManager_BP.ConstructionManager_BP_C" _defaultspawntransform "AlwaysSpawn" 0 _self 0))
      (Variables|Rererences|SetConstructionManagerRef _returnvalue))
    (:then_2
      (bind _returnvalue_2 (Game|SpawnActorfromClass "/Game/RTS_Game/Blueprints/Buldings/GhostBulding_Bp.GhostBulding_Bp_C" _defaultspawntransform "AlwaysSpawn" 0 _self 0))
      (Variables|Rererences|SetGhostBuildingRef _returnvalue_2))
    (:then_3
      (Input|SetInputModeGameandUI _self 0 "DoNotLock" false)
      (Utilities|CreateHuds)
      (UserInterface|Viewport|AddtoViewport (Variables|Rererences|GetMainHudRef) 0))))

(event EventTick
  (params (DeltaSeconds :type Float%20%28single-precision%29))
  (if (Variables|Default|GetBuildModeActive)
    (|SetCursorWorldPosition)))

(event Input|ActionEvents|InputActionPan
  (params (Key :type Key%20Structure))
  (bind _camerapawnref (Variables|Rererences|GetCameraPawnRef))
  (bind _returnvalue (Transformation|GetActorRotation _camerapawnref))
  (bind (_roll _pitch _yaw) (Math|Rotator|BreakRotator _returnvalue))
  ;[1 0 0.1752] Camera Movment
  ;;[1 1 1] Pan Y
  (:Pressed
    (Variables|Default|SetDisableCamNav true)
    (Utilities|FlowControl|Gate true) ; enters at Open
  )
  (:Released
    (Variables|Default|SetDisableCamNav false)
    (Utilities|FlowControl|Gate true) ; enters at Close
  ))

(event Input|ActionEvents|InputActionDeselect
  (params (Key :type Key%20Structure))
  ;[0.8702 1 0.2124] Construction Events
  (:Pressed
    (if (Variables|Default|GetBuildModeActive)
      (Default|KillGhost (Variables|Rererences|GetGhostBuildingRef))
      (Variables|Default|SetBuildModeActive false))))

(event Input|ActionEvents|InputActionPanReset
  (params (Key :type Key%20Structure))
  (bind _camerapawnref (Variables|Rererences|GetCameraPawnRef))
  (bind _returnvalue (Transformation|GetActorRotation _camerapawnref))
  (bind (_roll _pitch _yaw) (Math|Rotator|BreakRotator _returnvalue))
  ;[1 0 0.1752] Camera Movment
  ;;[1 1 1] Pan Reset
  (:Pressed
    (Transformation|SetActorRotation _camerapawnref (Math|Rotator|MakeRotator _roll 0.0 _yaw))))

(event Input|ActionEvents|InputActionZoomIn
  (params (Key :type Key%20Structure))
  (bind _camerapawnref (Variables|Rererences|GetCameraPawnRef))
  (bind _springarm (Variables|/Game/RTS_Game/Blueprints/CameraPawn.CameraPawn_C|GetSpringArm _camerapawnref))
  ;[1 0 0.1752] Camera Movment
  ;;[1 1 1] Zoom In/Out
  (:Pressed
    (Variables|/Script/Engine.SpringArmComponent|SetTargetArmLength _springarm (Math|Float|Clamp(Float) (- (Variables|/Script/Engine.SpringArmComponent|GetTargetArmLength _springarm) (Variables|Default|GetZoomSensitivity)) 5e+02 (Variables|Default|GetMaxArmDistance)))))

(event Input|ActionEvents|InputActionZoomOut
  (params (Key :type Key%20Structure))
  (bind _camerapawnref (Variables|Rererences|GetCameraPawnRef))
  (bind _springarm (Variables|/Game/RTS_Game/Blueprints/CameraPawn.CameraPawn_C|GetSpringArm _camerapawnref))
  ;[1 0 0.1752] Camera Movment
  ;;[1 1 1] Zoom In/Out
  (:Pressed
    (Variables|/Script/Engine.SpringArmComponent|SetTargetArmLength _springarm (Math|Float|Clamp(Float) (+ (Variables|Default|GetZoomSensitivity) (Variables|/Script/Engine.SpringArmComponent|GetTargetArmLength _springarm)) 5e+02 (Variables|Default|GetMaxArmDistance)))))

(event Input|ActionEvents|InputActionRotateBuldingRight
  (params (Key :type Key%20Structure))
  (bind _ghostbuildingref (Variables|Rererences|GetGhostBuildingRef))
  (bind _returnvalue (Transformation|GetActorRotation _ghostbuildingref))
  ;[0.8702 1 0.2124] Construction Events
  (:Pressed
    (if (and (Utilities|IsValid (Variables|Rererences|GetGhostBuildingRef)) (Variables|Default|GetBuildModeActive))
      (Transformation|SetActorRotation _ghostbuildingref (Math|Rotator|MakeRotator (.roll _returnvalue) (.pitch _returnvalue) (- (.yaw _returnvalue) (Variables|Default|GetBuildingRotationRate)))))))

(event Input|ActionEvents|InputActionRotateBuldingLEft
  (params (Key :type Key%20Structure))
  (bind _ghostbuildingref (Variables|Rererences|GetGhostBuildingRef))
  (bind _returnvalue (Transformation|GetActorRotation _ghostbuildingref))
  ;[0.8702 1 0.2124] Construction Events
  (:Pressed
    (if (and (Utilities|IsValid (Variables|Rererences|GetGhostBuildingRef)) (Variables|Default|GetBuildModeActive))
      (Transformation|SetActorRotation _ghostbuildingref (Math|Rotator|MakeRotator (.roll _returnvalue) (.pitch _returnvalue) (+ (.yaw _returnvalue) (Variables|Default|GetBuildingRotationRate)))))))

(event Input|ActionEvents|InputActionPan
  (params (Key :type Key%20Structure))
  (bind _camerapawnref (Variables|Rererences|GetCameraPawnRef))
  (bind _returnvalue (Transformation|GetActorRotation _camerapawnref))
  (bind (_roll _pitch _yaw) (Math|Rotator|BreakRotator _returnvalue))
  ;[1 0 0.1752] Camera Movment
  ;;[1 1 1] PanX
  (:Pressed
    (Variables|Default|SetDisableCamNav true)
    (Utilities|FlowControl|Gate true) ; enters at Open
  )
  (:Released
    (Variables|Default|SetDisableCamNav false)
    (Utilities|FlowControl|Gate true) ; enters at Close
  ))

(event Input|AxisEvents|InputAxisMoveForward
  (params (AxisValue :type Float%20%28single-precision%29))
  ;[1 0 0.1752] Camera Movment
  ;;[1 1 1] Movement X
  (if (not (Variables|Default|GetDisableCamNav))
    (Transformation|SetActorTransform (Variables|Rererences|GetCameraPawnRef) (Utilities|MovementX (CallFunction|MovementSpeedCalculation) (Variables|Default|GetFastMoveMultiplier) AxisValue (Variables|Rererences|GetCameraPawnRef)))))

(event Input|AxisEvents|InputAxisMoveRight
  (params (AxisValue :type Float%20%28single-precision%29))
  (bind _movesensitivity (CallFunction|MovementSpeedCalculation))
  (bind _camerapawnref (Variables|Rererences|GetCameraPawnRef))
  (bind _fastmovemultiplier (Variables|Default|GetFastMoveMultiplier))
  (bind _transform (Utilities|MovementY _movesensitivity AxisValue _fastmovemultiplier _camerapawnref))
  (bind (_location _rotation _scale) (Math|Transform|BreakTransform _transform))
  (bind (_x _y) (Math|Vector|BreakVector _location))
  ;[1 0 0.1752] Camera Movment
  ;;[1 1 1] Movement Y
  (if (not (Variables|Default|GetDisableCamNav))
    (Transformation|SetActorTransform (Variables|Rererences|GetCameraPawnRef) (Math|Transform|MakeTransform (Math|Vector|MakeVector _x _y 1e+02) _rotation _scale))))

(event Input|MouseEvents|MouseX
  (params (AxisValue :type Float%20%28single-precision%29))
  (bind _camerapawnref (Variables|Rererences|GetCameraPawnRef))
  (bind _returnvalue (Transformation|GetActorRotation _camerapawnref))
  (bind (_roll _pitch _yaw) (Math|Rotator|BreakRotator _returnvalue))
  ;[1 0 0.1752] Camera Movment
  ;;[1 1 1] PanX
  (Utilities|FlowControl|Gate true
    (:Exit
      (Transformation|SetActorRotation (Variables|Rererences|GetCameraPawnRef) (Math|Rotator|MakeRotator _roll _pitch (+ _yaw (* AxisValue (Variables|Default|GetPanSensitivity))))))))

(event Input|MouseEvents|MouseY
  (params (AxisValue :type Float%20%28single-precision%29))
  ;[1 0 0.1752] Camera Movment
  ;;[1 1 1] Edge Movement
  (if (not (Variables|Default|GetDisableCamNav))
    (Utilities|ScreenEdgeMovment) ; enters at MouseY
  ))

(event Input|MouseEvents|MouseX
  (params (AxisValue :type Float%20%28single-precision%29))
  ;[1 0 0.1752] Camera Movment
  ;;[1 1 1] Edge Movement
  (if (not (Variables|Default|GetDisableCamNav))
    (bind (_deltaxspeed _deltayspeed) (Utilities|ScreenEdgeMovment))
    (Transformation|AddActorLocalOffset (Variables|Rererences|GetCameraPawnRef) (Math|Vector|MakeVector _deltaxspeed _deltayspeed 0.0) true false)))

(event Input|MouseEvents|MouseY
  (params (AxisValue :type Float%20%28single-precision%29))
  (bind _camerapawnref (Variables|Rererences|GetCameraPawnRef))
  (bind _returnvalue (Transformation|GetActorRotation _camerapawnref))
  (bind (_roll _pitch _yaw) (Math|Rotator|BreakRotator _returnvalue))
  ;[1 0 0.1752] Camera Movment
  ;;[1 1 1] Pan Y
  (Utilities|FlowControl|Gate true
    (:Exit
      (Transformation|SetActorRotation (Variables|Rererences|GetCameraPawnRef) (Math|Rotator|MakeRotator _roll (Math|Float|Clamp(Float) (+ _pitch (* AxisValue (Variables|Default|GetPanSensitivity))) -15.0 45.0) _yaw)))))

(event Input|KeyboardEvents|LeftShift
  (params (Key :type Key%20Structure))
  ;[1 0 0.1752] Camera Movment
  ;;[1 1 1] Move Multiplier
  (:Pressed
    (Variables|Default|SetFastMoveMultiplier 2.0))
  (:Released
    (Variables|Default|SetFastMoveMultiplier 1.0)))

(event Input|MouseEvents|LeftMouseButton
  (params (Key :type Key%20Structure))
  ;[0.8702 1 0.2124] Construction Events
  (:Pressed
    (if (|VerifyAsPlaceable)
      (bind _constructionstruct (Default|GetConstructionStruct (Variables|Rererences|GetGhostBuildingRef)))
      (Default|QueueConstruction (Variables|Rererences|GetConstructionManagerRef) _constructionstruct)
      (Default|KillGhost (Variables|Rererences|GetGhostBuildingRef)))))

(event Input|KeyboardEvents|V
  (params (Key :type Key%20Structure))
  (bind _self self)
  (bind _sightdistance (Variables|Default|GetSightDistance))
  (bind _mouselocation (CallFunction|SetCursorWorldPosition _self _sightdistance))
  (:Pressed
    (Variables|Default|Setpizda true)
    (if (Variables|Default|Getpizda) :!label _label
      (Game|SpawnActorfromClass "/Game/RTS_Game/Blueprints/AI/NPC_BP.NPC_BP_C" (Math|Transform|MakeTransform (Math|Vector|MakeVector (.x _mouselocation) (.y _mouselocation) 93.0) "0, 0, 0" "0.250000,0.250000,0.250000") "Undefined" 0 0)))
  (:Released
    (Variables|Default|Setpizda false)
    (goto _label)))

(fn ConstructionScript)

(fn MovementSpeedCalculation
  (return (Math|Float|Clamp(Float) (/ (Variables|/Script/Engine.SpringArmComponent|GetTargetArmLength (Variables|/Game/RTS_Game/Blueprints/CameraPawn.CameraPawn_C|GetSpringArm (Variables|Rererences|GetCameraPawnRef))) 1e+02) 5.0 2e+01)))

(fn SetSightDistance
  (return (+ (Variables|Default|GetSightDistance) (Variables|/Script/Engine.SpringArmComponent|GetTargetArmLength (Variables|/Game/RTS_Game/Blueprints/CameraPawn.CameraPawn_C|GetSpringArm (Variables|Rererences|GetCameraPawnRef))))))

(fn SetCallendar
  (params (Date :type Array%20of%20Integers))
  (return false))

(fn SetClock
  (params (Time :type Array%20of%20Integers))
  (return false))
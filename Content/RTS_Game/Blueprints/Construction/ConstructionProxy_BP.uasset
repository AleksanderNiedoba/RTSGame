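; ConstructionProxy_BP is the ghost-material stand-in for a building under construction in the RTS.
; Reported workers scale progress by dividing the game-state time unit, which follows game speed events, and work accrues each tick toward the construction time.
; A camera-facing widget above the mesh shows percentage progress.
; On completion it fires ConstructionCompleted, frees and unhides its workers, then destroys itself after a short delay.
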(event Custom|AdjustTime
  (params (TimeUnit :type Float%20%28single-precision%29))
  (Variables|Default|SetTimeUnit TimeUnit))

(event EventBeginPlay
  (bind _output_get (Variables|References|SetGameStateRef (.AsMy%20Game%20State (Utilities|Casting|CastToMyGameState (Game|GetGameState)))))
  (Variables|Default|SetTimeUnit (Variables|/Game/RTS_Game/GameBP/MyGameState.MyGameState_C|GetTimeUnit _output_get))
  (EventDispatchers|BindEventtoUpdateGameSpeed _output_get (EventDispatchers|CreateEvent :!event Custom|AdjustTime)))

(event EventTick
  (params (DeltaSeconds :type Float%20%28single-precision%29))
  (bind _worktimespent (Variables|Default|GetWorkTimeSpent))
  (bind _constructiontime (Variables|Default|GetConstructionTime))
  (Variables|Default|SetDelta DeltaSeconds)
  (if (not (Variables|Default|GetIsConstructionCompleted))
    (CallFunction|DoWork)
    (CallFunction|UpdateConstructionTimeLeft _worktimespent _constructiontime)
    (if (>= _worktimespent _constructiontime)
      (Variables|Default|SetIsConstructionCompleted true)
      (Default|CallConstructionCompleted self)
      (CallFunction|ConstructionComplete)
      (Utilities|FlowControl|Delay 0.2)
      (Actor|DestroyActor))))

(fn ConstructionScript
  (bind _returnvalue (Transformation|GetActorLocation))
  (bind _staticmesh (Variables|Default|GetStaticMesh))
  (Components|StaticMesh|SetStaticMesh _staticmesh (Variables|Default|GetDisplayMesh))
  (Rendering|Material|SetMaterial _staticmesh 0 "/Game/RTS_Game/Materials/Ghost_M_Inst.Ghost_M_Inst")
  (Transformation|SetWorldLocation (Variables|Default|GetWidget) (Math|Vector|MakeVector (.x _returnvalue) (.y _returnvalue) (+ (.z (.boxextent (StaticMesh|GetBounds (Variables|Default|GetDisplayMesh)))) 1e+02)) false false)
  (CallFunction|SetBuildingEntrence (Variables|Default|GetEntrence) (Variables|Default|GetStaticMesh))
  (CallFunction|SetBuildingCollisonBox (Variables|Default|GetBox) (Variables|Default|GetStaticMesh)))

(fn SetConstructionTime
  (params (WorkHours :type Float%20%28single-precision%29))
  (Variables|Default|SetConstructionTime (* WorkHours 6e+01))
  (return))

(fn DoWork
  (bind _activeworkres (CallFunction|GetWorkforce))
  (if (> _activeworkres 0.0)
    (bind _output_get (Variables|Default|SetClockWork (.ClockWorkOut (CallFunction|SetClockWork (Variables|Default|GetDelta) (/ (Variables|Default|GetTimeUnit) _activeworkres) (Variables|Default|GetClockWork)))))
    (Variables|Default|SetWorkTimeSpent (* _output_get 6e+01))
    (return)
    (else
      (return))))

(fn UpdateConstructionTimeLeft
  (params (WorkTimeSpent :type Float%20%28single-precision%29) (ConstructionTime :type Float%20%28single-precision%29))
  (bind _widget (Variables|Default|GetWidget))
  (bind _astime_displayer (Utilities|Casting|CastToTimeDisplayer (UserInterface|GetUserWidgetObject _widget)))
  (Default|SetDisplayTime _astime_displayer (CallFunction|GetPercentageText WorkTimeSpent ConstructionTime))
  (Transformation|SetWorldRotation _widget (Math|Rotator|FindLookatRotation (Transformation|GetWorldLocation _widget) (Camera|GetCameraLocation (Game|GetPlayerCameraManager 0))) false false))

(fn GetWorkforce
  (return (Math|Conversions|ToFloat(Integer) (Utilities|Array|Length (Variables|Default|GetActiveWorkers)))))

(fn ReporttoShift
  (params (Worker :type NPC%20BP%20Object%20Reference))
  (Utilities|Array|Add (Variables|Default|GetActiveWorkers) Worker)
  (return))

(fn ConstructionComplete
  (if (> (CallFunction|GetWorkforce) 0.0)
    (for _array_element (Variables|Default|GetActiveWorkers)
      (Default|SetIsBusy _array_element false)
      (Rendering|SetActorHiddenInGame _array_element false))
    (Variables|Default|SetActiveWorkers (Utilities|Array|MakeArray 0))
    (return)
    (else
      (return))))